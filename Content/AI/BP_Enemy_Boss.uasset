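; Boss enemy Blueprint that extends a parent class and shows a boss health bar when the player reaches it.
; On BeginPlay it runs the parent logic, then stores world locations for the sword trace start and end points once.
; When a BP_ThirdPersonCharacter overlaps BossTrigger, it creates a WB_BossHealth widget on screen and hands its bar to BPCStats.
; The trigger has no guard, so each new overlap adds another widget.
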(event OnComponentBeginOverlap(BossTrigger)
  (params (OverlappedComponent :type Primitive%20Component%20Object%20Reference) (OtherActor :type Actor%20Object%20Reference) (OtherComp :type Primitive%20Component%20Object%20Reference) (OtherBodyIndex :type Integer) (bFromSweep :type Boolean) (SweepResult :type Hit%20Result%20Structure%20%28by%20ref%29))
  (Utilities|Casting|CastToBP_ThirdPersonCharacter OtherActor)
  (bind _returnvalue (UserInterface|CreateWidget "/Game/UI/WB_BossHealth.WB_BossHealth_C"))
  (bind _output_get (Variables|Default|SetBoss%20Health%20Widget _returnvalue))
  (UserInterface|Viewport|AddtoViewport _output_get 0)
  (Default|SetHealthProgressBar (Variables|Default|GetBPC_Stats) (Variables|/Game/UI/WB_BossHealth.WB_BossHealth_C|GetHealthBar (Variables|Default|GetBoss%20Health%20Widget))))

(event EventBeginPlay
  (|CallParentFunction)
  (Variables|Default|SetbossStartSwordTracePos (Transformation|GetWorldLocation (Variables|Default|GetBoss%20Start%20Sword%20Trace%20Pos)))
  (Variables|Default|SetbossEndSwordTracePos (Transformation|GetWorldLocation (Variables|Default|GetBoss%20End%20Sword%20Trace%20Pos))))

(event Collision|EventActorBeginOverlap
  (params (OtherActor :type Actor%20Object%20Reference)))

(event EventTick
  (params (DeltaSeconds :type Float%20%28single-precision%29)))

(fn ConstructionScript
  (|CallParentFunction))